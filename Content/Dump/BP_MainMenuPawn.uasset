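; BP_MainMenuPawn is the main menu pawn, driving the cinematic transitions into and out of the menu with level sequences.
; On BeginPlay it plays MM_Intro, and on finish it shows the widget switcher held by BP_MainMenuGamemode's widget and destroys the sequence actor.
; The Plyr event plays MM_Outro with the player hidden and paused at the end, then a finish callback opens the IntroPlayer level.
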(event `self.ReceiveBeginPlay`
  (bind (_outactor _returnvalue) (`LevelSequencePlayer.CreateLevelSequencePlayer` "/Game/Dump/Levels/MM_Intro.MM_Intro" (make `MovieSceneSequencePlaybackSettings` true)))
  (add `MovieSceneSequencePlayer.OnFinished` _returnvalue (delegate `OF`)))

(event `OF`
  (bind (_asbp_main_menu_gamemode _bsuccess) (cast `/Game/Dump/BP_MainMenuGamemode` (`GameplayStatics.GetGameMode`) :!pure true))
  (if _bsuccess
    (`Widget.SetVisibility` (`/Game/Dump/BP_MainMenu.WidgetSwitcher_40` (`/Game/Dump/BP_MainMenuGamemode.Widget` _asbp_main_menu_gamemode)) "Visible")
    (`self.K2_DestroyActor` (stale `self.ReceiveBeginPlay` _outactor))))

(event `Plyr`
  (bind (_outactor _returnvalue) (`LevelSequencePlayer.CreateLevelSequencePlayer` "/Game/Dump/Levels/MM_Outro.MM_Outro" (make `MovieSceneSequencePlaybackSettings` true (struct) (struct :`bAllowRounding` true) 1.0 0.0 false false false true false false "None" true)))
  (add `MovieSceneSequencePlayer.OnFinished` _returnvalue (delegate `goto`)))

(event `goto`
  (`GameplayStatics.OpenLevelBySoftObjectPtr` "/Game/Dump/IntroPlayer.IntroPlayer"))

(fn `UserConstructionScript`)