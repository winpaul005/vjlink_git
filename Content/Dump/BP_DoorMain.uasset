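; BP_DoorMain is a keycard-locked door actor that the player opens and closes through an inventory item callback.
; CallbackEvent receives an inventory slot index, checks that the player's item there is "keycard_noob", and otherwise has BP_Player speak a hint line.
; A valid card toggles IsOpen and slides DoorPlaceholder to or from its offset with MoveComponentTo, while IsMoving blocks retriggering during the move.
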(event `self.CallbackEvent`
  (params (CacheInventoryItemId :type Integer))
  (bind _returnvalue (`GameplayStatics.GetPlayerPawn` 0))
  (if (>= CacheInventoryItemId 0)
    (bind _asbp_player (cast `/Game/Dump/BP_Player` _returnvalue))
    (`KismetSystemLibrary.LogString` "Open")
    (if (`KismetStringLibrary.EqualEqual_StrStr` (`.ItemID` (break `InventorySlot` (`|GetArrayItem` (`C_InventoryComponent.InventoryArray` (`C_PlayerCharacter.InventoryComponent` _asbp_player)) CacheInventoryItemId))) "keycard_noob")
      (if (not (`self.Is Moving`))
        (set `self.Is Moving` true)
        (if (`self.Is Open`)
          (set `self.Is Open` false)
          (`KismetSystemLibrary.MoveComponentTo` (`self.doorPlaceholder`) (0.0 0.0 0.0) (struct) false false 8.0)
          (else
            (set `self.Is Open` true)
            (`KismetSystemLibrary.MoveComponentTo` (`self.doorPlaceholder`) (0.0 1680.0 0.0) (struct) false false 8.0)))
        (set `self.Is Moving` false))
      (else
        (`/Game/Dump/BP_Player.Talk` _asbp_player "Nothing significant happened..." 3.0)))
    (else
      (bind _asbp_player_2 (cast `/Game/Dump/BP_Player` _returnvalue))
      (`/Game/Dump/BP_Player.Talk` _asbp_player_2 "Looks like a keycard reader." 3.0))))

(fn `UserConstructionScript`
  (`parent.UserConstructionScript`))