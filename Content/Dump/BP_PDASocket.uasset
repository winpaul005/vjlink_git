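; BP_PDASocket is an item-use socket where the player plugs in a PDA and then obtains an upgraded one.
; Using a "pda" item consumes it, shows its mesh on the socket and runs the linked BP_RepairScreen monitor.
; Once plugged, using a "keyring" item consumes it, adds "betterpda" to the player's inventory and destroys the socket mesh component.
; IsPlugged and IsFinished flags sequence the two stages.
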(event `self.ReceiveBeginPlay`
  (add `self.OnUseItem` (delegate `Run`)))

(event `Run` :!signature `self.OnUseItem`
  (params (CacheInventoryItemId :type Integer))
  (bind _asbp_player (cast `/Game/Dump/BP_Player` (`GameplayStatics.GetPlayerPawn` 0)))
  (if (`self.IsPlugged`)
    (bind _inventorycomponent (`C_PlayerCharacter.InventoryComponent` _asbp_player))
    (bind _inventoryarray (`C_InventoryComponent.InventoryArray` _inventorycomponent))
    (bind _output_itemid (break `InventorySlot` (`|GetArrayItem` _inventoryarray CacheInventoryItemId)))
    (if (and (`KismetStringLibrary.EqualEqual_StrStr` _output_itemid "keyring") (not (`self.IsFinished`)))
      (`KismetArrayLibrary.Array_Remove` _inventoryarray CacheInventoryItemId)
      (`C_InventoryComponent.AddToInventory` _inventorycomponent "betterpda")
      (set `self.IsFinished` true)
      (`ActorComponent.K2_DestroyComponent` (`self.peck`)))
    (elif (`KismetStringLibrary.EqualEqual_StrStr` _output_itemid "pda")
      (`KismetArrayLibrary.Array_Remove` _inventoryarray CacheInventoryItemId)
      (`StaticMeshComponent.SetStaticMesh` (`self.peck`) "/Game/Dump/Levels/maynlevel/pda/pda.pda")
      (bind _asbp_repair_screen (cast `/Game/Dump/BP_RepairScreen` (`self.Monitor`)))
      (`/Game/Dump/BP_RepairScreen.Run` _asbp_repair_screen)
      (set `self.IsPlugged` true))))

(fn `UserConstructionScript`)