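; Player Blueprint handling movement feedback, a knife jab and links to the main UI and HUD.
; Move input sets BobFactor and swaps idle and run camera shakes for head bob, while a looping timer plays footsteps when moving and alive.
; Once widgets load, it fades in BP_MainUI, caches the HUD for speech lines and refreshes the game mode's seed.
; The knife briefly shows and slides the dagger, and Rumble plays a timed explosion shake.
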(event `self.ReceiveBeginPlay`
  (bind _mediaplayer (`self.MediaPlayer`))
  (`KismetSystemLibrary.ExecuteConsoleCommand` "stat FPS" null)
  (`SceneComponent.SetVisibility` (`self.dagger`) false false)
  (`MediaPlayer.SetLooping` _mediaplayer true)
  (`MediaPlayer.OpenSource` _mediaplayer "/Game/Movies/static.static")
  (add `self.WidgetInitCompleted` (delegate `WhenLoaded`))
  (`PlayerController.ClientStartCameraShake` :`self` (`GameplayStatics.GetPlayerController` 0) :`Shake` "/Game/Dump/BP_CameraShake.BP_CameraShake_C" :`Scale` (`self.BobFactor`))
  (`KismetSystemLibrary.K2_SetTimerDelegate` (delegate `walk`) (- (* (`self.BobFactor`) 1.7) (`self.BobFactor`)) true))

(event `walk`
  (if (> (`self.BobFactor`) 1.0)
    (if (not (<= (`self.Health`) 0.0))
      (`GameplayStatics.PlaySoundAtLocation` "/Game/Dump/Sounds/footsteps.footsteps" (`SceneComponent.K2_GetComponentLocation` (`self.CapsuleComponent`)) (struct) 1.0 1.0 0.0 null null null null))))

(event `WhenLoaded`
  (`KismetSystemLibrary.LogString` "Establishing Battlefield ctrl, stand by...")
  (bind _asbp_main_ui (cast `/Game/Dump/BP_MainUI` (`self.Player_Widget`))
    (:`then`
      (bind _output_get (set `self.As BP Main UI` _asbp_main_ui))
      (`/Game/Dump/BP_MainUI.Fade` _output_get true)
      (bind _asbp_hud (cast `/Game/Dump/BP_HUD` (`WidgetSwitcher.GetWidgetAtIndex` (`/Game/Dump/BP_MainUI.WidgetSwitcher_0` _output_get) 0))
        (:`then`
          (set `self.As BP HUD` _asbp_hud))
        (:`CastFailed`
          (`KismetSystemLibrary.LogString` "Sorgy")))
      (bind _asbp_neu_gamemode (cast `/Game/Dump/BP_NeuGamemode` (`GameplayStatics.GetGameMode`)))
      (bind _output_get_2 (set `self.As BP Neu Gamemode` _asbp_neu_gamemode))
      (`C_GameMode.RefreshSeed` _output_get_2))
    (:`CastFailed`
      (`KismetSystemLibrary.LogString` "Sorgy"))))

(event `Talk`
  (params (Speech :type String) (Duration :type "Float (double-precision)"))
  (`/Game/Dump/BP_HUD.SaySomething` (`self.As BP HUD`) Speech Duration))

(event `EnhancedInput|/Game/Dump/IA_Move`
  (params (ActionValue :type "Vector2D Structure") (ElapsedSeconds :type "Float (double-precision)") (TriggeredSeconds :type "Float (double-precision)") (InputAction :type "InputAction Object Reference" :default "/Game/Dump/IA_Move.IA_Move"))
  (bind _returnvalue (`GameplayStatics.GetPlayerController` 0))
  (bind _returnvalue_2 (`GameplayStatics.GetPlayerController` 0))
  (:`Started`
    (if (not (`self.bIsInventoryOpen`))
      (set `self.BobFactor` (`KismetMathLibrary.FMax` (`KismetMathLibrary.Abs` (* ActionValue_X 9.0)) (`KismetMathLibrary.Abs` (* ActionValue_Y 9.0))))
      (`PlayerController.ClientStopCameraShake` _returnvalue "/Game/Dump/BP_CameraShake.BP_CameraShake_C" false)
      (`PlayerController.ClientStartCameraShake` :`self` _returnvalue :`Shake` "/Game/Dump/BP_RunShake.BP_RunShake_C" :`Scale` (`self.BobFactor`))
      (else
        (set `self.BobFactor` 1.0 :!label _label)
        (`PlayerController.ClientStopCameraShake` _returnvalue_2 "/Game/Dump/BP_RunShake.BP_RunShake_C" false)
        (if (not (<= (`self.Health`) 0.0))
          (`PlayerController.ClientStartCameraShake` :`self` _returnvalue_2 :`Shake` "/Game/Dump/BP_CameraShake.BP_CameraShake_C" :`Scale` (`self.BobFactor`))))))
  (:`Completed`
    (goto _label)))

(event `Rumble`
  (params (Time :type "Float (double-precision)"))
  (bind _returnvalue (`GameplayStatics.GetPlayerController` 0))
  (`GameplayStatics.PlaySound2D` "/Game/Dump/Sounds/110111__ryansnook__big-explosion.110111__ryansnook__big-explosion" 1.0 1.0 0.0 null null)
  (`PlayerController.ClientStartCameraShake` :`self` _returnvalue :`Shake` "/Game/Dump/BP_Rumble.BP_Rumble_C")
  (`KismetSystemLibrary.Delay` Time)
  (`PlayerController.ClientStopCameraShake` _returnvalue "/Game/Dump/BP_Rumble.BP_Rumble_C" false))

(event `EnhancedInput|/Game/Dump/IA_Knife`
  (params (ActionValue :type Boolean) (ElapsedSeconds :type "Float (double-precision)") (TriggeredSeconds :type "Float (double-precision)") (InputAction :type "InputAction Object Reference" :default "/Game/Dump/IA_Knife.IA_Knife"))
  (bind _knifesock (`self.knifeSock`))
  (:`Started`
    (if (not (`self.IsKnifed`))
      (`SceneComponent.SetVisibility` (`self.dagger`) true false)
      (set `self.IsKnifed` true)
      (`KismetSystemLibrary.MoveComponentTo` _knifesock (4.0 0.0 -5.0) (struct) true true 0.1)
      (`KismetSystemLibrary.MoveComponentTo` _knifesock (-11.0 0.0 -5.0) (struct) true true 0.1)
      (set `self.IsKnifed` false)
      (`SceneComponent.SetVisibility` (`self.dagger`) false false))))

(fn `UserConstructionScript`)