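; Main menu game mode that handles starting the game, quitting and switching between menu pages.
; On BeginPlay it shows the cursor, sets Game and UI input, and caches the BP_MainMenu widget from the widget component on the placed Bp_mainmenu actor.
; PlayGame switches the widget switcher to its second page, waits briefly, then opens the Pr1 level.
; GotoWidge sets the switcher to any given page index.
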(event `self.ReceiveBeginPlay`
  (bind _returnvalue (`GameplayStatics.GetPlayerController` 0))
  (set `PlayerController.bShowMouseCursor` true _returnvalue)
  (`WidgetBlueprintLibrary.SetInputMode_GameAndUIEx` _returnvalue null)
  (bind _returnvalue_2 (`GameplayStatics.GetActorOfClass` "/Game/Dump/Levels/bp_mainmenu.bp_mainmenu_C"))
  (bind _asbp_main_menu (cast `/Game/Dump/BP_MainMenu` (`WidgetComponent.GetWidget` (`/Game/Dump/Levels/bp_mainmenu.Widget` _returnvalue_2))))
  (set `self.Widget` _asbp_main_menu))

(event `PlayGame`
  (`WidgetSwitcher.SetActiveWidgetIndex` (`/Game/Dump/BP_MainMenu.WidgetSwitcher_40` (`self.Widget`)) 1)
  (`KismetSystemLibrary.Delay` 0.3)
  (`GameplayStatics.OpenLevelBySoftObjectPtr` "/Game/Dump/Levels/PR1/pr1.pr1"))

(event `QuitGame`
  (`KismetSystemLibrary.QuitGame` null "Quit"))

(event `GotoWidge`
  (params (Index :type Integer))
  (`WidgetSwitcher.SetActiveWidgetIndex` (`/Game/Dump/BP_MainMenu.WidgetSwitcher_40` (`self.Widget`)) Index))

(fn `UserConstructionScript`)