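; BP_DoorGate is a gate in the VDNKh level that the player raises and lowers with a keycard from the inventory.
; CallbackEvent receives an inventory slot index and checks that item's ID on the player's InventoryComponent.
; The "keycard_noob" item toggles a timed vertical move of the Cube component, with IsOpen tracking state and IsMoving blocking retriggers.
; The PDA triggers an insufficient-clearance line through the player's Talk, and other items a "Nothing happened" line.
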(event `self.CallbackEvent`
  (params (CacheInventoryItemId :type Integer))
  (if (> CacheInventoryItemId -1)
    (bind _asbp_player (cast `/Game/Dump/BP_Player` (`GameplayStatics.GetPlayerPawn` 0)))
    (bind _output_get (set `self.As BP Player` _asbp_player))
    (bind _itemid (break `InventorySlot` (`|GetArrayItem` (`C_InventoryComponent.InventoryArray` (`C_PlayerCharacter.InventoryComponent` _output_get)) CacheInventoryItemId)))
    (if (`KismetStringLibrary.EqualEqual_StrStr` _itemid "pda")
      (`/Game/Dump/BP_Player.Talk` (`self.As BP Player`) "INSUFFICIENT CLEARANCE: Current clearance level: 1. Required clearance level: 2" 3.0)
      (elif (`KismetStringLibrary.EqualEqual_StrStr` _itemid "keycard_noob")
        (if (`self.Is Moving`)
          _
          (elif (`self.Is Open`)
            (set `self.Is Moving` true)
            (`KismetSystemLibrary.MoveComponentTo` (`self.Cube`) (0.0 0.0 0.0) (struct) false false 8.0)
            (set `self.Is Moving` false)
            (set `self.Is Open` false)
            (else
              (set `self.Is Moving` true)
              (`KismetSystemLibrary.MoveComponentTo` (`self.Cube`) (0.0 0.0 1500.0) (struct) false false 8.0)
              (set `self.Is Moving` false)
              (set `self.Is Open` true))))
        (else
          (`/Game/Dump/BP_Player.Talk` (`self.As BP Player`) "Nothing happened..." 3.0))))))

(fn `UserConstructionScript`
  (`parent.UserConstructionScript`))