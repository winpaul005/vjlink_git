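; BP_PickablePDA is a usable world actor that lets the player pick up a PDA.
; On BeginPlay it binds to the use-item event; the handler casts the player pawn to BP_Player and checks that InvnentorySize is above zero.
; If so, the player speaks a line about the PDA's previous holder, "pda" is added to the inventory and the actor destroys itself.
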(event `self.ReceiveBeginPlay`
  (add `self.OnUseItem` (delegate `OnUse`)))

(event `OnUse` :!signature `self.OnUseItem`
  (params (CacheInventoryItemId :type Integer))
  (bind _asbp_player (cast `/Game/Dump/BP_Player` (`GameplayStatics.GetPlayerPawn` 0)))
  (if (> (`C_InventoryComponent.InvnentorySize` (`C_PlayerCharacter.InventoryComponent` _asbp_player)) 0)
    (`/Game/Dump/BP_Player.Talk` _asbp_player "It's a wonder it's still operational. Let's just hope that... Alex Parker or whoever the original holder of this PDA is is at better place... On the other hand, will they be allowed to this \"better place\" after... all this..." 6.0)
    (`C_InventoryComponent.AddToInventory` (`C_PlayerCharacter.InventoryComponent` _asbp_player) "pda")
    (`self.K2_DestroyActor`)))

(fn `UserConstructionScript`)