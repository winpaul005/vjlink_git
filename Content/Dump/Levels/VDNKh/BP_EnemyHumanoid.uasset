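; Humanoid enemy that launches BP_KnifeAttacc at the player while its AI notices them.
; Tick polls the AI controller's Blackboard key IsNoticing and spawns the knife at Socket, rotated toward the player's capsule, passing itself as launcher.
; IsDormant acts as the ready flag: it clears on each throw and returns after a one-second Delay, or immediately once noticing stops.
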(event `self.ReceiveBeginPlay`
  (if (`self.Is Dormant`)
    _))

(event `self.ReceiveTick`
  (params (DeltaSeconds :type "Float (single-precision)"))
  (bind _returnvalue_location (`KismetMathLibrary.BreakTransform` (`SceneComponent.K2_GetComponentToWorld` (`self.Socket`))))
  (bind (_returnvalue_x _returnvalue_y _returnvalue_z) (`KismetMathLibrary.BreakVector` (`SceneComponent.K2_GetComponentLocation` (`Character.CapsuleComponent` (`GameplayStatics.GetPlayerCharacter` 0)))))
  (bind _output_get (set `self.IsNoticingBP` (`BlackboardComponent.GetValueAsBool` (`AIBlueprintHelperLibrary.GetBlackboard` (`AIBlueprintHelperLibrary.GetAIController` self)) "IsNoticing")))
  (if _output_get
    (if (`self.Is Dormant`)
      (set `self.Is Dormant` false)
      (`|SpawnActorFromClass` "/Game/Dump/BP_KnifeAttacc.BP_KnifeAttacc_C" (`KismetMathLibrary.MakeTransform` _returnvalue_location (`KismetMathLibrary.FindLookAtRotation` _returnvalue_location (`KismetMathLibrary.MakeVector` _returnvalue_x _returnvalue_y _returnvalue_z))) "Undefined" "MultiplyWithRoot" null self null)
      (`KismetSystemLibrary.Delay` 1.0)
      (set `self.Is Dormant` true)
      (elif (not (and (`self.IsNoticingBP`) (not (`self.Is Dormant`))))
        (set `self.Is Dormant` true)))
    (else
      (set `self.Is Dormant` true))))

(fn `UserConstructionScript`)