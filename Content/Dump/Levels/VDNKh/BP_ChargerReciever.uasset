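; BP_ChargerReciever is an interactable that recharges the player's flashlight from a limited TotalCharge pool.
; CallbackEvent rejects inventory items with a spoken line; otherwise it tops up the flashlight via AddCharge when charge remains.
; The remaining percentage is written to the bound BP_Charger's text render.
; When the pool cannot fill the flashlight, TotalCharge is zeroed before AddCharge reads it, so that branch adds nothing.
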(event `self.ReceiveBeginPlay`
  (`parent.ReceiveBeginPlay`))

(event `self.CallbackEvent`
  (params (CacheInventoryItemId :type Integer))
  (bind _returnvalue (/ (`KismetMathLibrary.Conv_IntToDouble` (`self.TotalCharge`)) 100.0))
  (bind _returnvalue_2 (- 1.0 (`C_PlayerCharacter.ChargeFlashlight` (`self.As BP Player_0`))))
  (bind _asbp_player (cast `/Game/Dump/BP_Player` (`GameplayStatics.GetPlayerPawn` 0)))
  (if (> CacheInventoryItemId -1)
    (`/Game/Dump/BP_Player.Talk` _asbp_player "Nothing happened." 3.0)
    (elif true
      (bind _output_get (set `self.As BP Player_0` _asbp_player))
      (if (< (`C_PlayerCharacter.ChargeFlashlight` _output_get) 1.0)
        (if (> (`self.TotalCharge`) 0)
          (if (> _returnvalue _returnvalue_2)
            (bind _output_get_2 (set `self.TotalCharge` (`KismetMathLibrary.FTrunc` (* (- _returnvalue _returnvalue_2) 100.0))))
            (`KismetSystemLibrary.LogString` (`KismetStringLibrary.Conv_IntToString` _output_get_2))
            (`C_PlayerCharacter.AddCharge` (`self.As BP Player_0`) _returnvalue_2)
            (else
              (set `self.TotalCharge` 0)
              (`C_PlayerCharacter.AddCharge` (`self.As BP Player_0`) _returnvalue)))
          (bind _asbp_charger (cast `/Game/Dump/Levels/VDNKh/BP_Charger` (`self.BindedItem`)))
          (`TextRenderComponent.K2_SetText` (`/Game/Dump/Levels/VDNKh/BP_Charger.TextRender` _asbp_charger) (`KismetTextLibrary.Conv_IntToText` (`self.TotalCharge`))))))))

(fn `UserConstructionScript`
  (`parent.UserConstructionScript`))