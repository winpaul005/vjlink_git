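; Keycard pickup for the VDNKh level that the player collects by using it.
; On BeginPlay it binds to the use-item event, then checks that the player's inventory size is above zero.
; If so, the player speaks a line and receives keycard_1 through the inventory component.
; The keycard then spawns BP_KeycardSceneTrigger at a hard-coded level transform and destroys itself.
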(event `self.ReceiveBeginPlay`
  (add `self.OnUseItem` (delegate `OnUse`)))

(event `OnUse` :!signature `self.OnUseItem`
  (params (CacheInventoryItemId :type Integer))
  (bind _asbp_player (cast `/Game/Dump/BP_Player` (`GameplayStatics.GetPlayerPawn` 0)))
  (if (> (`C_InventoryComponent.InvnentorySize` (`C_PlayerCharacter.InventoryComponent` _asbp_player)) 0)
    (`/Game/Dump/BP_Player.Talk` _asbp_player "At least something, I thought that I'm stuck here forever." 4.0)
    (`C_InventoryComponent.AddToInventory` (`C_PlayerCharacter.InventoryComponent` _asbp_player) "keycard_1")
    (`|SpawnActorFromClass` "/Game/Dump/Levels/maynlevel/BP_KeycardSceneTrigger.BP_KeycardSceneTrigger_C" (`KismetMathLibrary.MakeTransform` (-4009.0 3710.0 -40.0) (struct :`Yaw` 90.0)) "Undefined" "MultiplyWithRoot" null null)
    (`self.K2_DestroyActor`)))

(fn `UserConstructionScript`)