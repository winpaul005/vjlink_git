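; BP_Sniper is a turret-like sniper actor that tracks the player with a laser and punches them when the beam hits.
; Each Tick it yaws at a fixed rate toward player pawn 0, choosing direction by a plain yaw comparison.
; A laser emitter spawns once on the Cube, with its beam running from the Arrow to a forward line trace's hit or end.
; Punch is called on BP_Player every frame the trace hits it.
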(event `self.ReceiveTick`
  (params (DeltaSeconds :type "Float (single-precision)"))
  (bind (_returnvalue_roll _returnvalue_pitch _returnvalue_yaw) (`KismetMathLibrary.BreakRotator` (`self.K2_GetActorRotation`)))
  (bind (_returnvalue_roll_2 _returnvalue_pitch_2 _returnvalue_yaw_2) (`KismetMathLibrary.BreakRotator` (`self.K2_GetActorRotation`)))
  (bind _arrow (`self.Arrow`))
  (bind _returnvalue_location (`KismetMathLibrary.BreakTransform` (`self.GetTransform` (`GameplayStatics.GetPlayerPawn` 0))))
  (bind _returnvalue (`SceneComponent.K2_GetComponentLocation` _arrow))
  (bind (_returnvalue_roll_3 _returnvalue_pitch_3 _returnvalue_yaw_3) (`KismetMathLibrary.BreakRotator` (`KismetMathLibrary.FindLookAtRotation` (`self.K2_GetActorLocation`) _returnvalue_location)))
  (if (< _returnvalue_yaw_2 _returnvalue_yaw_3)
    (set `self.DirectionInt` 1)
    (elif (> _returnvalue_yaw_2 _returnvalue_yaw_3)
      (set `self.DirectionInt` -1)
      (else
        (set `self.DirectionInt` 0))))
  (`self.K2_SetActorRotation` (`KismetMathLibrary.MakeRotator` _returnvalue_roll _returnvalue_pitch (+ _returnvalue_yaw (* (* 50.0 DeltaSeconds) (`self.DirectionInt`)))))
  (`|ExecutionSequence`
    (:`then_0`
      (`/Engine/EditorBlueprintResources/StandardMacros.DoOnce` false
        (:`Completed`
          (bind _returnvalue_2 (`GameplayStatics.SpawnEmitterAttached` "/Game/Dump/Levels/VDNKh/P_Laser.P_Laser" (`self.Cube`)))
          (set `self.PartLaser` _returnvalue_2))))
    (:`then_1`
      (`ParticleSystemComponent.SetBeamSourcePoint` (`self.PartLaser`) 0 _returnvalue 0)
      (bind _outhit (`KismetSystemLibrary.LineTraceSingle` _returnvalue (+ _returnvalue (* (`SceneComponent.GetForwardVector` _arrow) 5000.0)) "TraceTypeQuery1"))
      (set `self.Out Hit Blocking Hit` (`GameplayStatics.BreakHitResult` _outhit))
      (set `self.Out Hit Hit Actor` (`.HitActor` (`GameplayStatics.BreakHitResult` _outhit)))
      (set `self.Out Hit Location` (`.Location` (`GameplayStatics.BreakHitResult` _outhit)))
      (`ParticleSystemComponent.SetBeamTargetPoint` (`self.PartLaser`) 0 (`KismetMathLibrary.SelectVector` (`self.Out Hit Location`) (`.TraceEnd` (`GameplayStatics.BreakHitResult` _outhit)) (`self.Out Hit Blocking Hit`)) 0)
      (bind _asbp_player (cast `/Game/Dump/BP_Player` (`self.Out Hit Hit Actor`)))
      (`C_PlayerCharacter.Punch` _asbp_player 1.0))))

(fn `UserConstructionScript`)