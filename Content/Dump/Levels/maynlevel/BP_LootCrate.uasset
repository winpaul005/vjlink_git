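; BP_LootCrate is a usable loot crate that opens an unlock widget when the player uses it.
; On use, if not yet breached, it unbinds its use event, disables the player's look and starts BP_Unlock's cycle with its reward and security level.
; The widget's success event removes the widget and marks the crate breached.
; The crate itself neither restores look nor rebinds use.
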(event `self.ReceiveBeginPlay`
  (add `self.OnUseItem` (delegate `OnUse`)))

(event `OnUse` :!signature `self.OnUseItem`
  (params (CacheInventoryItemId :type Integer))
  (if (not (`self.IsBreached`))
    (clear `self.OnUseItem`)
    (bind _asbp_player (cast `/Game/Dump/BP_Player` (`GameplayStatics.GetPlayerPawn` 0)))
    (set `C_PlayerCharacter.bCanLook` false _asbp_player)
    (bind _returnvalue (`|CreateWidget` "/Game/Dump/BP_Unlock.BP_Unlock_C"))
    (`UserWidget.AddToViewport` _returnvalue 0)
    (`/Game/Dump/BP_Unlock.StartCycle` _returnvalue (`self.Reward`) (`self.SecurityLvl`))
    (add `/Game/Dump/BP_Unlock.OnSucc` _returnvalue (delegate `ClerAll`))))

(event `ClerAll`
  (`Widget.RemoveFromParent` (stale `OnUse` _returnvalue))
  (set `self.IsBreached` true))

(fn `UserConstructionScript`)