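; BP_TransitionSector is a trigger actor that spawns a random level section when the player overlaps it.
; It picks a row from the LevelSections data table using the random stream held by BP_NeuGamemode, so selection follows that shared stream.
; The row's LevelInstance class is spawned at the trigger's root location and rotation, then the trigger destroys itself.
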(event `self.ReceiveActorBeginOverlap`
  (params (OtherActor :type "Actor Object Reference"))
  (bind _defaultsceneroot (`self.DefaultSceneRoot`))
  (bind _asbp_player (cast `/Game/Dump/BP_Player` OtherActor))
  (if (`KismetSystemLibrary.IsValid` _asbp_player)
    (bind _asbp_neu_gamemode (cast `/Game/Dump/BP_NeuGamemode` (`GameplayStatics.GetGameMode`)))
    (bind _outrownames (`DataTableFunctionLibrary.GetDataTableRowNames` "/Game/Dump/Levels/LevelSections.LevelSections"))
    (bind _returnvalue (- (`KismetArrayLibrary.Array_Length` _outrownames) 0))
    (`KismetSystemLibrary.LogString` (`KismetStringLibrary.Conv_IntToString` _returnvalue))
    (bind _returnvalue_2 (`|GetDataTableRow` "/Game/Dump/Levels/LevelSections.LevelSections" (`|GetArrayItem` _outrownames (`KismetMathLibrary.RandomIntegerFromStream` (`C_GameMode.RandomStream` _asbp_neu_gamemode) _returnvalue)))
      (:`then`
        (`|SpawnActorFromClass` (`.LevelInstance_3_155A779D4EC8C726AA5EADA0FB81D986` (break `/Game/Dump/Levels/Level` _returnvalue_2)) (`KismetMathLibrary.MakeTransform` (`SceneComponent.K2_GetComponentLocation` _defaultsceneroot) (`SceneComponent.K2_GetComponentRotation` _defaultsceneroot)) "Undefined" "MultiplyWithRoot" null null)
        (`self.K2_DestroyActor`)))))

(fn `UserConstructionScript`)