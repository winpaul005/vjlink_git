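; BP_MainGateTrigger is an overlap trigger that fires the main gate's finale when the player crosses it.
; On a BP_Player overlap it unbinds its Box's begin-overlap events, destroys the BP_Roaster, maxes HUD "Severeness" and rumbles the player.
; It spawns a BP_HallwayBlocker at a hardcoded location, then, if GateBP is valid, calls GrandFinale and destroys itself.
; Non-player overlaps print an error.
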(event `self.ReceiveActorBeginOverlap`
  (params (OtherActor :type "Actor Object Reference"))
  (bind _asbp_player (cast `/Game/Dump/BP_Player` OtherActor)
    (:`then`
      (clear `PrimitiveComponent.OnComponentBeginOverlap` (`self.Box`))
      (bind _returnvalue (`GameplayStatics.GetActorOfClass` "/Game/Dump/Levels/maynlevel/entities/BP_Roaster.BP_Roaster_C"))
      (`self.K2_DestroyActor` _returnvalue)
      (`KismetMaterialLibrary.SetScalarParameterValue` "/Game/HUDProperties.HUDProperties" "Severeness" 1.0)
      (`/Game/Dump/BP_Player.Rumble` _asbp_player 0.8)
      (`|SpawnActorFromClass` "/Game/Dump/Levels/maynlevel/BP_HallwayBlocker.BP_HallwayBlocker_C" (`KismetMathLibrary.MakeTransform` (-1020.0 1380.0 -30.0)) "Undefined" "MultiplyWithRoot" null null)
      (bind _gatebp (`self.GateBP`)
        (:`then`
          (`/Game/Dump/Levels/maynlevel/BP_FinaleDemoGate.GrandFinale` _gatebp)
          (`self.K2_DestroyActor`))
        (:`else`)))
    (:`CastFailed`
      (`KismetSystemLibrary.PrintText` "ERROR: What has crossed is not player. SORGY!"))))

(fn `UserConstructionScript`)