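; BP_RestorelightScene is a one-shot trigger actor that restores scene lighting when the player enters it.
; On actor overlap with BP_Player, it loops through AvailibleLights and sets each referenced light to its paired intensity, instantly, since the Lerp alpha is fixed at 1.
; It unbinds the Box's begin-overlap events beforehand and destroys the Box afterwards.
; Any other overlapping actor only prints an error message.
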(event `self.ReceiveActorBeginOverlap`
  (params (OtherActor :type "Actor Object Reference"))
  (cast `/Game/Dump/BP_Player` OtherActor
    (:`then`
      (clear `PrimitiveComponent.OnComponentBeginOverlap` (`self.Box`))
      (for _array_element (`self.Availible Lights`)
        (`LightComponent.SetIntensity` (break `/Game/Dump/Light_comp` _array_element) (`KismetMathLibrary.Lerp` (`LightComponentBase.Intensity` (break `/Game/Dump/Light_comp` _array_element)) (`.intensity_5_9DB53A4A482F23D50D01E88459BA53D7` (break `/Game/Dump/Light_comp` _array_element)) 1.0)))
      (`ActorComponent.K2_DestroyComponent` (`self.Box`)))
    (:`CastFailed`
      (`KismetSystemLibrary.PrintText` "ERROR: What has crossed is not player. SORGY!"))))

(fn `UserConstructionScript`)