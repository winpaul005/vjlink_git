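; BP_RemovableVent is a vent hatch that the player can remove by using a screwdriver from the inventory.
; On BeginPlay it binds its Use event to OnUseItem, which looks up the passed inventory index in BP_Player's InventoryComponent.
; A screwdriver detaches the hatch mesh with physics enabled, is removed from the inventory and is reported broken through the player's Talk.
; Any other item triggers a spoken hint about the screws.
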(event `self.ReceiveBeginPlay`
  (add `self.OnUseItem` (delegate `Use`)))

(event `Use` :!signature `self.OnUseItem`
  (params (CacheInventoryItemId :type Integer))
  (bind _vent_hatch_uvfix (`self.vent_hatch_uvfix`))
  (set `self.Cache Inventory Item Id` CacheInventoryItemId)
  (bind _asbp_player (cast `/Game/Dump/BP_Player` (`GameplayStatics.GetPlayerPawn` 0)))
  (bind _inventorycomponent (`C_PlayerCharacter.InventoryComponent` _asbp_player))
  (set `self.Inventory Component` _inventorycomponent)
  (bind _output_itemid (break `InventorySlot` (`|GetArrayItem` (`C_InventoryComponent.InventoryArray` _inventorycomponent) (`self.Cache Inventory Item Id`))))
  (if (`KismetStringLibrary.EqualEqual_StrStr` _output_itemid "screwdriver")
    (`PrimitiveComponent.SetSimulatePhysics` _vent_hatch_uvfix true)
    (`SceneComponent.K2_DetachFromComponent` _vent_hatch_uvfix "KeepRelative" "KeepRelative" "KeepRelative" true)
    (`KismetArrayLibrary.Array_Remove` (`C_InventoryComponent.InventoryArray` (`self.Inventory Component`)) (`self.Cache Inventory Item Id`))
    (`/Game/Dump/BP_Player.Talk` _asbp_player "Screwdriver broke." 3.0)
    (else
      (`/Game/Dump/BP_Player.Talk` _asbp_player "Won't budge, there must be a way to remove those screws..." 4.0))))

(fn `UserConstructionScript`)