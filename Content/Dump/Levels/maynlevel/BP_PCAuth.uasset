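; Computer authentication actor that unlocks a PC screen when the player uses the right inventory item on it.
; On BeginPlay it binds Auth to its OnUseItem event and caches the BP_ComputerWidget from its widget component.
; Auth looks up the used slot in the player's inventory: the better PDA calls Login, while any other item registers a failed attempt.
; The basic PDA also makes the player voice an exasperated line.
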(event `self.ReceiveBeginPlay`
  (add `self.OnUseItem` (delegate `Auth`))
  (bind _asbp_computer_widget (cast `/Game/Dump/Levels/maynlevel/BP_ComputerWidget` (`WidgetComponent.GetWidget` (`self.Widget`))))
  (set `self.As BP Computer Widget` _asbp_computer_widget))

(event `Auth` :!signature `self.OnUseItem`
  (params (CacheInventoryItemId :type Integer))
  (bind _as_bp_computer_widget (`self.As BP Computer Widget`))
  (bind _asbp_player (cast `/Game/Dump/BP_Player` (`GameplayStatics.GetPlayerPawn` 0)))
  (bind _output_itemid (break `InventorySlot` (`|GetArrayItem` (`C_InventoryComponent.InventoryArray` (`C_PlayerCharacter.InventoryComponent` _asbp_player)) CacheInventoryItemId)))
  (if (`KismetStringLibrary.EqualEqual_StrStr` _output_itemid "betterpda")
    (`/Game/Dump/Levels/maynlevel/BP_ComputerWidget.Login` _as_bp_computer_widget)
    (else
      (if (`KismetStringLibrary.EqualEqual_StrStr` _output_itemid "pda")
        (`/Game/Dump/BP_Player.Talk` _asbp_player "You gotta be kidding me... WHAT ELSE DO YOU NEED?!" 3.0))
      (`/Game/Dump/Levels/maynlevel/BP_ComputerWidget.Attempt` _as_bp_computer_widget false))))

(fn `UserConstructionScript`)