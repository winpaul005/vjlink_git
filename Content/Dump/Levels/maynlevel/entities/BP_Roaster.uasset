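; BP_Roaster is a hostile entity that turns to face the player and hurts them when seen with clear line of sight.
; Unless Tren is set, Tick traces to the camera, eases the HUD "Severeness" parameter by visibility, and applies frame-scaled damage via Punch while recently rendered.
; Overlapping it deals a heavy Punch.
; Using the "GFYS" item relocates it and spawns a BP_TPTrigger targeting it.
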(event `self.ReceiveBeginPlay`
  (bind _returnvalue (`GameplayStatics.GetActorOfClass` "/Script/Engine.PostProcessVolume"))
  (bind _aspost_process_volume (cast `PostProcessVolume` _returnvalue))
  (set `self.As Post Process Volume` _aspost_process_volume)
  (bind _outactors (`GameplayStatics.GetAllActorsOfClass` "/Script/vjlink.C_UseableItem"))
  (for _array_element _outactors
    (if (`KismetStringLibrary.EqualEqual_StrStr` (`C_UseableItem.EventId` _array_element) "GFYS")
      (set `self.Trigger Alarm` _array_element)))
  (bind _asbp_player (cast `/Game/Dump/BP_Player` (`GameplayStatics.GetPlayerPawn` 0)))
  (set `self.As BP Player` _asbp_player)
  (add `C_UseableItem.OnUseItem` (`self.Trigger Alarm`) (delegate `SurpriseMF`)))

(event `SurpriseMF`
  (params (CacheInventoryItemId :type Integer))
  (`self.K2_SetActorLocation` (-350.0 7470.0 750.0))
  (bind _returnvalue (`|SpawnActorFromClass` "/Game/Dump/Levels/maynlevel/BP_TPTrigger.BP_TPTrigger_C" (`KismetMathLibrary.MakeTransform` (1200.0 4840.0 190.0) (struct :`Yaw` 90.0)) "Undefined" "MultiplyWithRoot" null null))
  (set `/Game/Dump/Levels/maynlevel/BP_TPTrigger.Victim Actor` self _returnvalue)
  (set `/Game/Dump/Levels/maynlevel/BP_TPTrigger.Transform` (1370.0 4360.0 210.0) _returnvalue))

(event `self.ReceiveActorBeginOverlap`
  (params (OtherActor :type "Actor Object Reference"))
  (bind _asbp_player (cast `/Game/Dump/BP_Player` OtherActor))
  (`C_PlayerCharacter.Punch` _asbp_player 228.0))

(event `self.ReceiveTick`
  (params (DeltaSeconds :type "Float (single-precision)"))
  (bind _as_bp_player (`self.As BP Player`))
  (bind _returnvalue_location (`KismetMathLibrary.BreakTransform` (`SceneComponent.K2_GetComponentToWorld` (`Actor.RootComponent` _as_bp_player))))
  (if (not (`self.bTren`))
    (bind (_outhit _returnvalue) (`KismetSystemLibrary.LineTraceSingle` (`self.K2_GetActorLocation`) (`SceneComponent.K2_GetComponentLocation` (`C_PlayerCharacter.MainCamera` (cast `/Game/Dump/BP_Player` (`GameplayStatics.GetPlayerPawn` 0) :!pure true))) "TraceTypeQuery1"))
    (if (not _returnvalue)
      (set `self.Triggered` true)
      (bind _returnvalue_2 (`KismetMaterialLibrary.GetScalarParameterValue` "/Game/HUDProperties.HUDProperties" "Severeness"))
      (`KismetMaterialLibrary.SetScalarParameterValue` "/Game/HUDProperties.HUDProperties" "Severeness" (`KismetMathLibrary.Lerp` _returnvalue_2 0.3 0.05))
      (if (`self.WasRecentlyRendered` self 0.2)
        (set `self.Triggered PLUS` true)
        (bind _returnvalue_3 (`KismetMaterialLibrary.GetScalarParameterValue` "/Game/HUDProperties.HUDProperties" "Severeness"))
        (`KismetMaterialLibrary.SetScalarParameterValue` "/Game/HUDProperties.HUDProperties" "Severeness" (`KismetMathLibrary.Lerp` _returnvalue_3 1.0 0.05))
        (`C_PlayerCharacter.Punch` _as_bp_player (* (`GameplayStatics.GetWorldDeltaSeconds`) (`self.Damage`)))
        (else
          (set `self.Triggered PLUS` false)))
      (else
        (set `self.Triggered` false)
        (bind _returnvalue_4 (`KismetMaterialLibrary.GetScalarParameterValue` "/Game/HUDProperties.HUDProperties" "Severeness"))
        (`KismetMaterialLibrary.SetScalarParameterValue` "/Game/HUDProperties.HUDProperties" "Severeness" (`KismetMathLibrary.Lerp` _returnvalue_4 0.1 0.05))))
    (`SceneComponent.K2_SetWorldRotation` (`self.DefaultSceneRoot`) (`KismetMathLibrary.MakeRotator` 0.0 0.0 (.yaw (`KismetMathLibrary.FindLookAtRotation` (`SceneComponent.K2_GetComponentLocation` (`self.DefaultSceneRoot`)) _returnvalue_location))) false false)))

(fn `UserConstructionScript`)