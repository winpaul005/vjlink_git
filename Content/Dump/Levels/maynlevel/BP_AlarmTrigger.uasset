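; BP_AlarmTrigger is a level trigger that sets off an alarm when BP_Player overlaps it.
; It plays the BeeDoo sound at its own location and teleports the first found BP_Roaster to a hard-coded position.
; It then spawns a BP_TPTrigger, passing it the roaster as VictimActor along with a preset transform.
; It also unbinds the Box's begin-overlap delegate, and non-player overlaps only print an error.
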(event `self.ReceiveActorBeginOverlap`
  (params (OtherActor :type "Actor Object Reference"))
  (cast `/Game/Dump/BP_Player` OtherActor
    (:`then`
      (clear `PrimitiveComponent.OnComponentBeginOverlap` (`self.Box`))
      (bind _returnvalue (`GameplayStatics.GetActorOfClass` "/Game/Dump/Levels/maynlevel/entities/BP_Roaster.BP_Roaster_C"))
      (`GameplayStatics.SpawnSoundAtLocation` "/Game/Dump/Sounds/BeeDoo.BeeDoo" (`SceneComponent.K2_GetComponentLocation` (`self.DefaultSceneRoot`)) (struct) 1.0 1.0 0.0 null null)
      (`self.K2_SetActorLocation` _returnvalue (-149.000001 7599.999999 822.0) false false)
      (bind _returnvalue_2 (`|SpawnActorFromClass` "/Game/Dump/Levels/maynlevel/BP_TPTrigger.BP_TPTrigger_C" (`KismetMathLibrary.MakeTransform` (1200.0 4840.0 190.0) (struct :`Yaw` 90.0)) "Undefined" "MultiplyWithRoot" null null))
      (set `/Game/Dump/Levels/maynlevel/BP_TPTrigger.Victim Actor` _returnvalue _returnvalue_2)
      (set `/Game/Dump/Levels/maynlevel/BP_TPTrigger.Transform` (1370.0 4360.0 210.0) _returnvalue_2))
    (:`CastFailed`
      (`KismetSystemLibrary.PrintText` "ERROR: What has crossed is not player. SORGY!"))))

(fn `UserConstructionScript`)