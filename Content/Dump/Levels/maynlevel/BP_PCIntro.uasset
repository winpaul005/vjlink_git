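; BP_PCIntro is an intro computer actor whose widget component displays a BP_IntroWidget.
; BeginPlay binds the Auth event to an on-use-item callback and caches the cast widget.
; Using an item triggers Auth, which calls Login on that widget regardless of the item ID.
; A separate Coitus event calls the widget's Prikku function; nothing in this graph invokes it.
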(event `self.ReceiveBeginPlay`
  (add `self.OnUseItem` (delegate `Auth`))
  (bind _asbp_intro_widget (cast `/Game/Dump/Levels/maynlevel/BP_IntroWidget` (`WidgetComponent.GetWidget` (`self.Widget`))))
  (set `self.As BP Computer Widget` _asbp_intro_widget))

(event `Auth` :!signature `self.OnUseItem`
  (params (CacheInventoryItemId :type Integer))
  (`/Game/Dump/Levels/maynlevel/BP_IntroWidget.Login` (`self.As BP Computer Widget`)))

(event `Coitus`
  (`/Game/Dump/Levels/maynlevel/BP_IntroWidget.Prikku` (`self.As BP Computer Widget`)))

(fn `UserConstructionScript`)