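; Keycard-locked sliding door that generates a random level section behind it when used.
; On item use, it compares the item ID's numeric suffix to ClearanceLevel, and the player speaks a refusal if too low.
; Non-sequence doors first spawn a LevelSections room via the game mode's random stream, destroying overlapping spawns.
; Door1 slides open with audio, then closes after a timeout if clear or on later end overlap.
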(event `Open` :!signature `self.OnUseItem`
  (params (CacheInventoryItemId :type Integer))
  (bind _box (`self.Box`))
  (bind _asbp_player (cast `/Game/Dump/BP_Player` (`GameplayStatics.GetPlayerPawn` 0)))
  (if (>= (`KismetStringLibrary.Conv_StringToInt` (`.RightS` (`KismetStringLibrary.Split` (`.ItemID` (break `InventorySlot` (`|GetArrayItem` (`C_InventoryComponent.InventoryArray` (`C_PlayerCharacter.InventoryComponent` _asbp_player)) CacheInventoryItemId))) "_"))) (`self.Clearance Level`))
    (if (`self.Sequence Door`)
      (if (not (`self.Is Open`)) :!label _label
        (if (not (`self.Is Moving`))
          (`AudioComponent.SetSound` (`self.Audio`) "/Game/Dump/Sounds/379803__mafon2__metal-door-groaning.379803__mafon2__metal-door-groaning")
          (`AudioComponent.Play` (`self.Audio`) 0.0)
          (set `self.Is Moving` true)
          (set `self.Is Open` true)
          (`KismetSystemLibrary.MoveComponentTo` (`self.door_1`) (0.0 -190.0 31.0) (struct) false false 0.8)
          (`AudioComponent.SetSound` (`self.Audio`) "/Game/Dump/Sounds/218723__bareform__bang-1.218723__bareform__bang-1")
          (set `self.Is Moving` false)
          (set `self.timerEnded` false)
          (`KismetSystemLibrary.Delay` (`self.TimeoutTime`))
          (set `self.timerEnded` true)
          (bind (_outactors _returnvalue) (`KismetSystemLibrary.ComponentOverlapActors` _box (`SceneComponent.K2_GetComponentToWorld` _box) (`|MakeArray` "ObjectTypeQuery3" :!type "EObjectTypeQuery Enum")))
          (if (not _returnvalue)
            (`AudioComponent.SetSound` (`self.Audio`) "/Game/Dump/Sounds/379803__mafon2__metal-door-groaning.379803__mafon2__metal-door-groaning")
            (`AudioComponent.Play` (`self.Audio`) 0.0)
            (`KismetSystemLibrary.MoveComponentTo` (`self.door_1`) (0.0 0.0 31.0) (struct) false false 0.8)
            (`AudioComponent.SetSound` (`self.Audio`) "/Game/Dump/Sounds/218723__bareform__bang-1.218723__bareform__bang-1")
            (set `self.Is Open` false))))
      (else
        (`self.SpawnRoom` (`GameplayStatics.GetPlayerPawn` 0))
        (if (`self.Has Spawned`)
          (goto _label))))
    (else
      (`/Game/Dump/BP_Player.Talk` _asbp_player "This door requires a level 3 or greater clearance" 3.0)
      (`/Game/Dump/BP_Player.Talk` _asbp_player "This door requires a level 3 or greater clearance" 3.0))))

(event `self.ReceiveBeginPlay`
  (add `self.OnUseItem` (delegate `Open`)))

(event `self.ReceiveActorEndOverlap`
  (params (OtherActor :type "Actor Object Reference"))
  (if (and (`self.Is Open`) (`self.timerEnded`))
    (`self.Open` 0)
    (if (not (`self.Is Moving`))
      (set `self.Is Moving` true)
      (`KismetSystemLibrary.MoveComponentTo` (`self.door_1`) (0.0 0.0 31.0) (struct) false false 0.8)
      (set `self.Is Moving` false)
      (set `self.Is Open` false))))

(fn `SpawnRoom`
  (params (`Other Act` :type "Actor Object Reference"))
  (returns (`Is Success` :type Boolean) (`Actor Return` :type "Actor Object Reference"))
  (bind _spawn (`self.spawn`))
  (bind _asbp_player (cast `/Game/Dump/BP_Player` `Other Act`))
  (`/Engine/EditorBlueprintResources/StandardMacros.IsValid` _asbp_player
    (:`Is Valid`
      (bind _asbp_neu_gamemode (cast `/Game/Dump/BP_NeuGamemode` (`GameplayStatics.GetGameMode`)))
      (bind _outrownames (`DataTableFunctionLibrary.GetDataTableRowNames` "/Game/Dump/Levels/LevelSections.LevelSections"))
      (bind _returnvalue (`KismetArrayLibrary.Array_Length` _outrownames))
      (`KismetSystemLibrary.LogString` (`KismetStringLibrary.Conv_IntToString` _returnvalue))
      (bind _returnvalue_2 (`|GetDataTableRow` "/Game/Dump/Levels/LevelSections.LevelSections" (`|GetArrayItem` _outrownames (`KismetMathLibrary.RandomIntegerFromStream` (`C_GameMode.RandomStream` _asbp_neu_gamemode) _returnvalue)))
        (:`then`
          (bind _returnvalue_3 (`|SpawnActorFromClass` (`.LevelInstance_3_155A779D4EC8C726AA5EADA0FB81D986` (break `/Game/Dump/Levels/Level` _returnvalue_2)) (`KismetMathLibrary.MakeTransform` (`SceneComponent.K2_GetComponentLocation` _spawn) (`SceneComponent.K2_GetComponentRotation` _spawn) (`SceneComponent.K2_GetComponentScale` _spawn)) "AdjustIfPossibleButDontSpawnIfColliding" "OverrideRootScale" null null))
          (bind _returnvalue_4 (`KismetSystemLibrary.IsValid` _returnvalue_3))
          (if (or (> (`KismetArrayLibrary.Array_Length` (`self.GetOverlappingActors` _returnvalue_3 null)) 0) (not _returnvalue_4))
            (`self.K2_DestroyActor` _returnvalue_3))
          (bind _output_get (set `self.Has Spawned` _returnvalue_4))
          (`KismetSystemLibrary.PrintText` (`KismetTextLibrary.Conv_BoolToText` _output_get))
          (set `self.Sequence Door` true)
          (return true _returnvalue_3))))))

(fn `UserConstructionScript`)