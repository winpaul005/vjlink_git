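; Finale gate for the demo level, ending the game with a staged gate sequence and a return to the main menu.
; GrandFinale switches the assigned lights to an orange warning look, rumbles the player and raises the HUD Severeness parameter.
; After timed delays, two gate halves move in two stages, finally sliding in opposite directions with another rumble and a UI fade.
; The fade-out animation's finish callback opens the main menu level.
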(event `self.ReceiveBeginPlay`
  (bind _asbp_player (cast `/Game/Dump/BP_Player` (`GameplayStatics.GetPlayerPawn` 0)))
  (set `self.As BP Player` _asbp_player))

(event `GrandFinale`
  (bind _as_bp_player (`self.As BP Player`))
  (bind _as_bp_main_ui (`/Game/Dump/BP_Player.As BP Main UI` _as_bp_player))
  (for _array_element (`self.Lights`)
    (bind _lightcomponent (`Light.LightComponent` _array_element))
    (`LightComponent.SetLightFunctionMaterial` _lightcomponent "/Game/Dump/Levels/maynlevel/MT_LightWarn.MT_LightWarn")
    (`LightComponent.SetLightColor` _lightcomponent (struct :`R` 1.0 :`G` 0.483935 :`A` 1.0) true)
    (`LightComponent.SetIntensity` _lightcomponent 1.0))
  (`/Game/Dump/BP_Player.Rumble` (`self.As BP Player`) 0.7)
  (`KismetMaterialLibrary.SetScalarParameterValue` "/Game/HUDProperties.HUDProperties" "Severeness" 1.0)
  (`KismetSystemLibrary.Delay` 3.0)
  (`|ExecutionSequence`
    (:`then_0`
      (`KismetSystemLibrary.MoveComponentTo` (`self.gates_gate_L`) (0.0 0.0 0.0) (struct) false false 3.0))
    (:`then_1`
      (`KismetSystemLibrary.MoveComponentTo` (`self.gates_bake`) (0.0 0.0 0.0) (struct) false false 3.0)))
  (`KismetSystemLibrary.Delay` 3.0)
  (`|ExecutionSequence`
    (:`then_0`
      (`KismetSystemLibrary.MoveComponentTo` (`self.gates_gate_L`) (0.0 62.0 0.0) (struct) false false 3.0))
    (:`then_1`
      (`KismetSystemLibrary.MoveComponentTo` (`self.gates_bake`) (0.0 -62.0 0.0) (struct) false false 3.0))
    (:`then_2`
      (`/Game/Dump/BP_Player.Rumble` _as_bp_player 2.5))
    (:`then_3`
      (`/Game/Dump/BP_MainUI.Fade` _as_bp_main_ui false)
      (`UserWidget.BindToAnimationFinished` _as_bp_main_ui (`/Game/Dump/BP_MainUI.FadeOut` _as_bp_main_ui) (delegate `HereIGo`)))))

(event `HereIGo`
  (`GameplayStatics.OpenLevelBySoftObjectPtr` "/Game/mainmenu.mainmenu"))

(fn `UserConstructionScript`)