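; One-shot level trigger, named for the keycard scene, that stages a light failure when BP_Player overlaps it.
; It gathers lights by scanning PointLight actors and every actor's LightComponents, then applies the MT_LightFailure light function.
; After a short delay it switches them to MT_Light; if IsLethal, it also zeroes their intensity and clears the player's flashlight-active flag.
; It then destroys itself.
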(event `self.ReceiveActorBeginOverlap`
  (params (OtherActor :type "Actor Object Reference"))
  (cast `/Game/Dump/BP_Player` OtherActor
    (:`then`
      (clear `PrimitiveComponent.OnComponentBeginOverlap` (`self.Box`))
      (bind _outactors (`GameplayStatics.GetAllActorsOfClass` "/Script/Engine.PointLight"))
      (for _array_element _outactors
        (`KismetArrayLibrary.Array_Add` (`self.Availible Lights`) (`Light.LightComponent` _array_element)))
      (bind _outactors_2 (`GameplayStatics.GetAllActorsOfClass` "/Script/Engine.Actor"))
      (for _array_element_2 _outactors_2
        (for _array_element_3 (`self.K2_GetComponentsByClass` _array_element_2 "/Script/Engine.LightComponent")
          (`KismetArrayLibrary.Array_Add` (`self.Availible Lights`) _array_element_3)))
      (for _array_element_4 (`self.Availible Lights`)
        (`LightComponent.SetLightFunctionMaterial` _array_element_4 "/Game/Dump/MT_LightFailure.MT_LightFailure"))
      (`KismetSystemLibrary.Delay` 3.0)
      (for _array_element_5 (`self.Availible Lights`)
        (if (`self.IsLethal`)
          (`LightComponent.SetIntensity` _array_element_5 (`KismetMathLibrary.Lerp` (`LightComponentBase.Intensity` _array_element_5) 0.0 1.0)))
        (`LightComponent.SetLightFunctionMaterial` _array_element_5 "/Game/Dump/Levels/VDNKh/MT_Light.MT_Light"))
      (bind _asbp_player (cast `/Game/Dump/BP_Player` (`GameplayStatics.GetPlayerPawn` 0))
        (:`then`
          (if (`self.IsLethal`)
            (set `C_PlayerCharacter.bIsFlashlightActive` false _asbp_player)))
        (:`CastFailed`
          _))
      (`self.K2_DestroyActor`))
    (:`CastFailed`
      (`KismetSystemLibrary.PrintText` "ERROR: What has crossed is not player. SORGY!"))))

(fn `UserConstructionScript`)