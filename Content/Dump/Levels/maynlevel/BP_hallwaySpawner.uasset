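; Hallway spawner that procedurally builds a branching level out of rooms on BeginPlay, starting at its own transform.
; Each pass spawns a random LevelSections table entry at every open transform, using the BP_NeuGamemode random stream.
; BP_DoorElevator child actors in the new sections supply the next pass's transforms through their Spawn components.
; MaximumRooms sets the number of passes rather than a room total; spawns adjust for collisions or are skipped.
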(event `self.ReceiveBeginPlay`
  (`KismetArrayLibrary.Array_Add` (`self.AvailibleTransforms`) (`self.GetTransform`))
  (`self.SpawnRoom`)
  (for _ (range (+ (`self.MaximumRooms`) 1))
    (`self.SpawnRoom`)))

(event `SpawnRoom`
  (bind _asbp_neu_gamemode (cast `/Game/Dump/BP_NeuGamemode` (`GameplayStatics.GetGameMode`)))
  (bind _outrownames (`DataTableFunctionLibrary.GetDataTableRowNames` "/Game/Dump/Levels/LevelSections.LevelSections"))
  (for _array_element (`self.AvailibleTransforms`)
    (bind _returnvalue (`|GetDataTableRow` "/Game/Dump/Levels/LevelSections.LevelSections" (`|GetArrayItem` _outrownames (`KismetMathLibrary.RandomIntegerFromStream` (`C_GameMode.RandomStream` _asbp_neu_gamemode) (`KismetArrayLibrary.Array_Length` _outrownames))))
      (:`then`
        (bind _returnvalue_2 (`|SpawnActorFromClass` (`.LevelInstance_3_155A779D4EC8C726AA5EADA0FB81D986` (break `/Game/Dump/Levels/Level` _returnvalue)) _array_element "AdjustIfPossibleButDontSpawnIfColliding" "MultiplyWithRoot" null null))
        (`KismetArrayLibrary.Array_Add` (`self.PotentialRapists`) _returnvalue_2))))
  (`KismetArrayLibrary.Array_Clear` (`self.AvailibleTransforms`))
  (for _array_element_2 (`self.PotentialRapists`)
    (for _array_element_3 (`self.GetAllChildActors` _array_element_2 true)
      (bind _asbp_door_elevator (cast `/Game/Dump/Levels/PR1/BP_DoorElevator` _array_element_3))
      (`KismetArrayLibrary.Array_Add` (`self.AvailibleTransforms`) (`SceneComponent.K2_GetComponentToWorld` (`/Game/Dump/Levels/PR1/BP_DoorElevator.spawn` _asbp_door_elevator)))))
  (`KismetArrayLibrary.Array_Clear` (`self.PotentialRapists`)))

(fn `UserConstructionScript`)