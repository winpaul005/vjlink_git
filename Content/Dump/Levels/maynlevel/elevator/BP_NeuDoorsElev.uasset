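; Sliding double elevator door that toggles open and closed when its bound use-item event fires.
; BeginPlay binds Opn to that event; the inventory item ID it receives is unused.
; Opn slides the two door meshes apart or back together with parallel MoveComponentTo calls, using IsMoving to ignore triggers mid-motion.
; A pawn overlap check is left unconnected and never runs.
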(event `Opn` :!signature `self.OnUseItem`
  (params (CacheInventoryItemId :type Integer))
  (if (not (`self.Is Open`))
    (if (not (`self.Is Moving`))
      (set `self.Is Moving` true)
      (set `self.Is Open` true)
      (`|ExecutionSequence`
        (:`then_0`
          (`KismetSystemLibrary.MoveComponentTo` (`self.elev_door1_UV1`) (0.0 100.0 0.0) (struct) false false 0.8)
          (set `self.Is Moving` false))
        (:`then_1`
          (`KismetSystemLibrary.MoveComponentTo` (`self.elev_door1_UV`) (0.0 -100.0 0.0) (struct) false false 0.8))))
    (elif (not (`self.Is Moving`))
      (set `self.Is Moving` true)
      (set `self.Is Open` false)
      (`|ExecutionSequence`
        (:`then_0`
          (`KismetSystemLibrary.MoveComponentTo` (`self.elev_door1_UV1`) (0.0 0.0 0.0) (struct) false false 0.8)
          (set `self.Is Moving` false))
        (:`then_1`
          (`KismetSystemLibrary.MoveComponentTo` (`self.elev_door1_UV`) (0.0 0.0 0.0) (struct) false false 0.8))))))

(event `self.ReceiveBeginPlay`
  (add `self.OnUseItem` (delegate `Opn`)))

(fn `UserConstructionScript`)