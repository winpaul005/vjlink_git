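; Toggleable door that swings open or closed when its use-item event fires.
; On BeginPlay it binds Open to OnUseItem; the passed inventory item ID is not checked.
; Open uses MoveComponentTo to rotate Door1 90 degrees or back over a short time, with IsMoving blocking input mid-motion and IsOpen tracking state.
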(event `self.ReceiveBeginPlay`
  (add `self.OnUseItem` (delegate `Open`)))

(event `Open` :!signature `self.OnUseItem`
  (params (CacheInventoryItemId :type Integer))
  (if (not (`self.Is Open`))
    (if (not (`self.Is Moving`))
      (set `self.Is Moving` true)
      (`KismetSystemLibrary.MoveComponentTo` (`self.door_1`) (0.0 0.0 0.0) (struct :`Yaw` -90.0) false false 0.8)
      (set `self.Is Moving` false)
      (set `self.Is Open` true))
    (elif (not (`self.Is Moving`))
      (set `self.Is Moving` true)
      (`KismetSystemLibrary.MoveComponentTo` (`self.door_1`) (0.0 0.0 0.0) (struct) false false 0.8)
      (set `self.Is Moving` false)
      (set `self.Is Open` false))))

(fn `UserConstructionScript`)