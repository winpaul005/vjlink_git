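; BP_VendingMachine is a one-time interactable vending machine that gives the player a soda.
; On BeginPlay it binds Use to the OnUseItem event and caches the BP_Player pawn.
; The first use makes the player remark on spending their only quarter, adds "soda" to their InventoryComponent and sets a Used flag.
; Later uses only make the player say they are out of cash.
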(event `self.ReceiveBeginPlay`
  (add `self.OnUseItem` (delegate `Use`))
  (bind _asbp_player (cast `/Game/Dump/BP_Player` (`GameplayStatics.GetPlayerPawn` 0)))
  (set `self.As BP Player` _asbp_player))

(event `Use` :!signature `self.OnUseItem`
  (params (CacheInventoryItemId :type Integer))
  (bind _as_bp_player (`self.As BP Player`))
  (if (`self.Used`)
    (`/Game/Dump/BP_Player.Talk` (`self.As BP Player`) "I'm out of cash." 3.0)
    (else
      (`/Game/Dump/BP_Player.Talk` _as_bp_player "Used the only quarter I had in my pockets. " 3.0)
      (`C_InventoryComponent.AddToInventory` (`C_PlayerCharacter.InventoryComponent` _as_bp_player) "soda")
      (set `self.Used` true))))

(fn `UserConstructionScript`)