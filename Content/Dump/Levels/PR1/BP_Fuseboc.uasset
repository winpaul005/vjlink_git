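; BP_Fuseboc is a level fuse box puzzle actor that the player sabotages with a soda item to open a linked gate.
; On BeginPlay it caches the player and binds Use to the item-use event.
; Soda triggers a player line, opens a valid Gate, destroys its Box, marks damage, unbinds overlap events and briefly plays an electrocution sound.
; Any other item makes the player remark that the lever is welded shut.
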(event `self.ReceiveBeginPlay`
  (add `self.OnUseItem` (delegate `Use`))
  (bind _asbp_player (cast `/Game/Dump/BP_Player` (`GameplayStatics.GetPlayerPawn` 0)))
  (bind _output_get (set `self.As BP Player` _asbp_player)))

(event `Use` :!signature `self.OnUseItem`
  (params (CacheInventoryItemId :type Integer))
  (bind _as_bp_player (`self.As BP Player`))
  (bind _output_itemid (break `InventorySlot` (`|GetArrayItem` (`C_InventoryComponent.InventoryArray` (`C_PlayerCharacter.InventoryComponent` (stale `self.ReceiveBeginPlay` _output_get))) CacheInventoryItemId)))
  (if (`KismetStringLibrary.EqualEqual_StrStr` _output_itemid "soda")
    (`/Game/Dump/BP_Player.Talk` _as_bp_player "This was a risky move, but I have no choice though." 3.0)
    (bind _gate (`self.Gate`)
      (:`then`
        (if (not (`/Game/Dump/Levels/PR1/BP_Checkpoint.IsOpen` _gate))
          (`/Game/Dump/Levels/PR1/BP_Checkpoint.Open` _gate))
        (set `self.IsDamaged` true)
        (`ActorComponent.K2_DestroyComponent` (`/Game/Dump/Levels/PR1/BP_Checkpoint.Box` _gate))
        (clear `Actor.OnActorBeginOverlap`)
        (clear `Actor.OnActorEndOverlap`)
        (bind _returnvalue (`GameplayStatics.SpawnSound2D` "/Game/Dump/Sounds/30933__aust_paul__electrocute.30933__aust_paul__electrocute" 1.0 1.0 0.0 null))
        (`KismetSystemLibrary.Delay` 0.5)
        (`AudioComponent.Stop` _returnvalue)
        (`ActorComponent.K2_DestroyComponent` _returnvalue))
      (:`else`))
    (else
      (`/Game/Dump/BP_Player.Talk` _as_bp_player "The lever is welded shut. Can't shut it down like that." 3.0))))

(fn `UserConstructionScript`)